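; Base_shotBP is a projectile actor for the weapon system's shot system.
; On hitting any actor other than its owner, it spawns a green explosion at the impact point, prints a debug "Hello" and destroys itself.
; Logic to set projectile movement and damage range from BaseShot structures, activate movement and self-destroy after a delay exists but is disconnected, so it never runs.
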(event EventBeginPlay)

(event Collision|EventHit
  (params (MyComp :type Primitive%20Component%20Object%20Reference) (Other :type Actor%20Object%20Reference) (OtherComp :type Primitive%20Component%20Object%20Reference) (bSelfMoved :type Boolean) (HitLocation :type Vector :default "0, 0, 0") (HitNormal :type Vector :default "0, 0, 0") (NormalImpulse :type Vector :default "0, 0, 0") (Hit :type Hit%20Result%20Structure%20%28by%20ref%29))
  (if (not (== Other (Components|GetOwner)))
    ;[0.8047 1 0 0.5] Event hit determines spawn location for impact effect
    (Effects|SpawnEmitteratLocation "/Game/WeaponSystem/Shoot_System_Derived/Particles/P_ExplosionGreen.P_ExplosionGreen" HitLocation "0, 0, 0" "1.000000,1.000000,1.000000" false)
    (Development|PrintString "Hello")
    (Actor|DestroyActor)))

(fn ConstructionScript)