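; Base weapon actor for a weapon system, taking its skeletal mesh and ammo and firing settings from WeaponStructure data.
; FireSystem branches on beam or projectile, clip or none, and single or continuous fire, returning updated ammo structs.
; Beam paths spawn actors at sockets, while projectile leaf functions are empty, as are Fire and Reload events.
; Tick drives a delayed auto-reload while not firing, either discarding or topping up the clip.
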(event Custom|AutoReload
  (if true
    (Utilities|AutoReloadDelay 0.0
      (:Then%28IsNotFiring%29
        (if true ; Uses Clip
          ;[0 0.7891 1] ThrowClip
          (if true
            (Reload|ThrowClip)
            (CallFunction|UpdateWeaponAmmo)
            (else
              (Reload|ReloadClip)
              (CallFunction|UpdateWeaponAmmo))))))))

(event Custom|UpdateWeapon_1
  (params (Weapon :type Base%20Weapon%20Structure%20Structure))
  ;[0.251 1 0] UpdateWeapon
  (Variables|Default|SetWeaponStructure Weapon))

(event EventBeginPlay
  ;[0 1 0.8594] SetSkeletalMesh
  ;;[0 1 0.5781] BeginPlay
  (Class|SkinnedMeshComponent|SetSkeletalMesh (Variables|Default|GetSkeletalMesh) (Utilities|GetSkeletalMesh) true))

(event EventTick
  (params (DeltaSeconds :type Float%20%28single-precision%29))
  ;[1 0.5391 0] EventTick
  (Variables|Default|SetTime (+ DeltaSeconds (Variables|Default|GetTime)))
  (CallFunction|AutoReload))

(event EventReload
  ;[0 0.3437 1] Reload
)

(event EventFire
  ;[1 0.8672 0] Comment
)

(fn ConstructionScript
  ;[0 1 0.6953] Set Skeletal Mesh
  (Class|SkinnedMeshComponent|SetSkeletalMesh (Variables|Default|GetSkeletalMesh) (Utilities|GetSkeletalMesh) true))

(fn FireBeamNoClip
  (params (FireStructure :type Fire%20Structure%20Structure))
  (if (.SingleFire (Utilities|Struct|BreakBaseFire (.Base_Fire (Utilities|Struct|BreakFireStructure FireStructure))))
    (bind _returnbaseammo (Beam|FireBeamNoClipSF FireStructure))
    (return (Utilities|UpdateAmmowithFire FireStructure _returnbaseammo))
    (else
      (bind _returnbaseammo_2 (Beam|FireBeamNoClipDPS FireStructure))
      (return (Utilities|UpdateAmmowithFire FireStructure _returnbaseammo_2)))))

(fn FireBeamNoClipDPS
  (params (FireStructure :type Fire%20Structure%20Structure))
  (bind (_base_fire _base_shotstructure _beams_structure _base_ammo) (Utilities|Struct|BreakFireStructure FireStructure))
  (bind _beams_shot (Utilities|Struct|BreakBeam_Structure _beams_structure))
  (bind (_decrement _second _beam) (Utilities|Struct|BreakBeam_Shot _beams_shot))
  (CallFunction|SpawnBeam _beam _beams_structure (.BoneName (Utilities|Struct|BreakBaseFire _base_fire)))
  (bind _returnvalue (CallFunction|DecrementPerS 0.0 _second _decrement (Math|Conversions|ToFloat(Integer) (.CurrentAmmo (Utilities|Struct|BreakBaseAmmo _base_ammo)))))
  (return (Utilities|UpdateAmmoBase (Math|Float|Truncate _returnvalue) _base_ammo)))

(fn FireBeamNoClipSF
  (params (FireStructure :type Fire%20Structure%20Structure))
  (bind (_base_fire _base_shotstructure _beams_structure _base_ammo) (Utilities|Struct|BreakFireStructure FireStructure))
  (bind _beams_shot (Utilities|Struct|BreakBeam_Structure _beams_structure))
  (bind (_decrement _second _beam) (Utilities|Struct|BreakBeam_Shot _beams_shot))
  (CallFunction|SpawnBeam _beam _beams_structure (.BoneName (Utilities|Struct|BreakBaseFire _base_fire)))
  (return (Utilities|UpdateAmmoBase (- (.CurrentAmmo (Utilities|Struct|BreakBaseAmmo _base_ammo)) (Math|Float|Truncate _decrement)) _base_ammo)))

(fn FireBeamSystem
  (params (FireStructure :type Fire%20Structure%20Structure))
  (if (.Clip (Utilities|Struct|BreakBaseClip (.Base_Clip (Utilities|Struct|BreakFireStructure FireStructure))))
    (bind _fire_structure (Beam|FireBeamClip FireStructure))
    (return _fire_structure)
    (else
      (bind _firestructurereturn (Beam|FireBeamNoClip FireStructure))
      (return _firestructurereturn))))

(fn FireBeamClip
  (params (FireStructure :type Fire%20Structure%20Structure))
  (if (.SingleFire (Utilities|Struct|BreakBaseFire (.Base_Fire (Utilities|Struct|BreakFireStructure FireStructure))))
    (bind _returnbaseclip (Beam|FireBeamClipSF FireStructure))
    (return (Utilities|UpdateClipwithFire FireStructure _returnbaseclip))
    (else
      (bind _returnbaseclip_2 (Beam|FireBeamClipDPS FireStructure))
      (return (Utilities|UpdateClipwithFire FireStructure _returnbaseclip_2)))))

(fn FireBeamClipDPS
  (params (FireStructure :type Fire%20Structure%20Structure))
  (bind (_base_fire _base_shotstructure _beams_structure _base_ammo _base_clip) (Utilities|Struct|BreakFireStructure FireStructure))
  (bind _beams_shot (Utilities|Struct|BreakBeam_Structure _beams_structure))
  (bind (_decrement _second _beam) (Utilities|Struct|BreakBeam_Shot _beams_shot))
  (CallFunction|SpawnBeam _beam _beams_structure (.BoneName (Utilities|Struct|BreakBaseFire _base_fire)))
  (bind _returnvalue (CallFunction|DecrementPerS 0.0 _second _decrement (Math|Conversions|ToFloat(Integer) (.CurrentClip (Utilities|Struct|BreakBaseClip _base_clip)))))
  (return (Utilities|UpdateAmmoClip (Math|Float|Truncate _returnvalue) _base_clip)))

(fn FireBeamClipSF
  (params (FireStructure :type Fire%20Structure%20Structure))
  (bind (_base_fire _base_shotstructure _beams_structure _base_ammo _base_clip) (Utilities|Struct|BreakFireStructure FireStructure))
  (bind _beams_shot (Utilities|Struct|BreakBeam_Structure _beams_structure))
  (bind (_decrement _second _beam) (Utilities|Struct|BreakBeam_Shot _beams_shot))
  (CallFunction|SpawnBeam _beam _beams_structure (.BoneName (Utilities|Struct|BreakBaseFire _base_fire)))
  (return (Utilities|UpdateAmmoClip (- (.CurrentClip (Utilities|Struct|BreakBaseClip _base_clip)) (Math|Float|Truncate _decrement)) _base_clip)))

(fn SpawnBeam
  (params (Class :type Actor%20Class%20Reference) (BeamStructure :type Beam%20Structure%20Structure) (InSocketName :type Name))
  ;[0 1 0.1797] Spawn And Send Variables to Beam
  (bind _returnvalue (Game|SpawnActorfromClass Class (Transformation|GetSocketTransform (Variables|Default|GetSkeletalMesh) InSocketName "RTS_World") "AlwaysSpawn" 0 0))
  (Utilities|FlowControl|Sequence
    (:then_0
      (Utilities|FlowControl|Sequence
        (:then_0
          (Utilities|IsValid _returnvalue))))
    (:then_1
      (Utilities|IsValid _returnvalue))))

(fn DecrementPerS
  (params (CurrentTime :type Float%20%28single-precision%29) (Duration :type Float%20%28single-precision%29) (Decrement :type Float%20%28single-precision%29) (Value :type Float%20%28single-precision%29) (Times :type Integer))
  (bind _returnvalue (Math|Conversions|ToFloat(Integer) Times))
  (bind _returnvalue_2 (* Decrement _returnvalue))
  (bind _returnvalue_3 (- Value _returnvalue_2))
  ;[1 0.8672 0] Delay
  (|SetBy-RefVar CurrentTime (- (Variables|Default|GetTime) (Variables|Default|GetTime)) :!label _label)
  (if (not (>= Duration CurrentTime))
    ;[0 0.3437 1] KeepTrackOfTimes
    (bind _result (Math|Integer|IncrementInt Times)
      (:%20%20
        (|SetBy-RefVar Times _result)
        (if (>= _returnvalue_3 0.0)
          (Utilities|FlowControl|Sequence
            (:then_0
              (return _returnvalue_3))
            (:then_1
              (goto _label))))))))

(fn SpawnProjectile
  (params (Class :type Actor%20Class%20Reference) (InSocketName :type Name) (Base%20Shot%20Structure :type Base%20Shot%20Structure%20Structure))
  ;[1 0.4219 0] Spawn And Send Variables to Projectile
  (bind _returnvalue (Game|SpawnActorfromClass Class (Transformation|GetSocketTransform (Variables|Default|GetSkeletalMesh) InSocketName "RTS_World") "AlwaysSpawn" 0 0))
  (Utilities|IsValid _returnvalue))

(fn FireSystem
  (params (FireStructure :type Fire%20Structure%20Structure))
  (if (.Beam (Utilities|Struct|BreakBaseFire (.Base_Fire (Utilities|Struct|BreakFireStructure FireStructure))))
    (bind _firestructurereturn (Beam|FireBeamSystem FireStructure))
    (return _firestructurereturn)
    (else
      (bind _returnfirestructure (Projectile|FireProjectileSystem FireStructure))
      (return _returnfirestructure))))

(fn FireProjectileSystem
  (params (FireStructure :type Fire%20Structure%20Structure))
  (if (.Clip (Utilities|Struct|BreakBaseClip (.Base_Clip (Utilities|Struct|BreakFireStructure FireStructure))))
    (bind _firestructure1 (Projectile|FireProjectileClip FireStructure))
    (return _firestructure1)
    (else
      (bind _firestructure1_2 (Projectile|FireProjectileNoClip FireStructure))
      (return _firestructure1_2))))

(fn ReloadSystem
  (params (FireStructure :type Fire%20Structure%20Structure%20%28by%20ref%29))
  (bind (_clip _throwclip) (Utilities|ReloadEssentials FireStructure))
  (if _clip ; Does it use a clip?
    (if _throwclip ; throw clip?
      (Reload|ThrowClip FireStructure)
      (else
        (Reload|ReloadClip FireStructure)))))

(fn UpdateWeaponAmmo
  (params (BaseWeaponStructure :type Base%20Weapon%20Structure%20Structure))
  (Utilities|FlowControl|Sequence
    (:then_0
      ;[1 0 0.9375] UpdateAmmo1
      (switch Utilities|FlowControl|Switch|SwitchonFireType "NewEnumerator0"))
    (:then_1
      ;[1 0 0.9375] UpdateAmmo2
      (switch Utilities|FlowControl|Switch|SwitchonFireType "NewEnumerator0"))
    (:then_2
      ;[1 0 0.9375] UpdateSpecialAmmo
      (switch Utilities|FlowControl|Switch|SwitchonFireType "NewEnumerator0"))))

(fn ThrowClip
  (params (FireStructureG :type Fire%20Structure%20Structure))
  (bind (_base_ammo _base_clip) (Utilities|GetAmmoandClip FireStructureG))
  (bind (_base_ammo_2 _base_clip_2) (Utilities|GetAmmoandClip FireStructureG))
  (bind (_base_ammo_3 _base_clip_3) (Utilities|GetAmmoandClip FireStructureG))
  (bind _base_ammo_4 (Utilities|GetAmmoandClip FireStructureG))
  ;[0 1 0.7891] CurrentAmmoMoreThanMaxClip
  (Utilities|>= (Math|Conversions|ToFloat(Integer) (.currentammo _base_ammo)) (Math|Conversions|ToFloat(Integer) (.maxclip _base_clip))
    (:true
      (return (Utilities|UpdateFireStructureAmmos FireStructureG (Utilities|AmmoandClipTOFire (Utilities|UpdateAmmoBase (- (.currentammo _base_ammo) (.maxclip _base_clip)) _base_ammo_3) (Utilities|UpdateAmmoClip (.maxclip _base_clip) _base_clip_3)))))
    (:false
      ;[1 0 0.4219] CurrentAmmoMoreThan0
      (Utilities|> (Math|Conversions|ToFloat(Integer) (.currentammo _base_ammo_4)) 0.0
        (:true
          (return (Utilities|UpdateFireStructureAmmos FireStructureG (Utilities|AmmoandClipTOFire (Utilities|UpdateAmmoBase 0 _base_ammo_2) (Utilities|UpdateAmmoClip (.currentammo _base_ammo_4) _base_clip_2)))))))))

(fn ReloadClip
  (params (FireStructure :type Fire%20Structure%20Structure))
  (bind (_base_fire _base_shotstructure _beams_structure) (Utilities|Struct|BreakFireStructure FireStructure))
  (bind (_base_fire_2 _base_shotstructure_2 _beams_structure_2) (Utilities|Struct|BreakFireStructure FireStructure))
  (bind (_base_ammo _base_clip) (Utilities|GetAmmoandClip FireStructure))
  (bind (_base_ammo_2 _base_clip_2) (Utilities|GetAmmoandClip FireStructure))
  ;[1 0 0.7734] CurrentAmmoMoreThanClip
  (Utilities|>= (Math|Conversions|ToFloat(Integer) (.currentammo _base_ammo_2)) (Math|Conversions|ToFloat(Integer) (.maxclip _base_clip_2))
    (:true
      (return (Utilities|Struct|MakeFireStructure _base_fire_2 _base_shotstructure_2 _beams_structure_2 (Utilities|Struct|MakeBaseAmmo (- (+ (.currentammo _base_ammo_2) (.currentclip _base_clip_2)) (.maxclip _base_clip_2)) (.maxammo _base_ammo_2)) (Utilities|Struct|MakeBaseClip (.clip _base_clip_2) (.maxclip _base_clip_2) (.maxclip _base_clip_2) (.throwclip _base_clip_2)))))
    (:false
      (return (Utilities|Struct|MakeFireStructure _base_fire _base_shotstructure _beams_structure (Utilities|Struct|MakeBaseAmmo 0 (.maxammo _base_ammo)) (Utilities|Struct|MakeBaseClip (.clip _base_clip) (.currentammo _base_ammo) (.maxclip _base_clip) (.throwclip _base_clip)))))))

(fn FireProjectileNoClip
  (params (FireStructure :type Fire%20Structure%20Structure))
  (if (.SingleFire (Utilities|Struct|BreakBaseFire (.Base_Fire (Utilities|Struct|BreakFireStructure FireStructure))))
    (bind _baseammoo (Projectile|FireProjectileNoClipSF FireStructure))
    (return (Utilities|UpdateAmmowithFire FireStructure _baseammoo))
    (else
      (bind _baseammo (Projectile|FireProjectileNoClipDPS FireStructure))
      (return (Utilities|UpdateAmmowithFire FireStructure _baseammo)))))

(fn FireProjectileClip
  (params (Firestructure :type Fire%20Structure%20Structure))
  (if (.SingleFire (Utilities|Struct|BreakBaseFire (.Base_Fire (Utilities|Struct|BreakFireStructure Firestructure))))
    (bind _baseclip (Projectile|FireProjectileClipSF Firestructure))
    (return (Utilities|UpdateClipwithFire Firestructure _baseclip))
    (else
      (bind _baseclip_2 (Projectile|FireProjectileClipDPS Firestructure))
      (return (Utilities|UpdateClipwithFire Firestructure _baseclip_2)))))

(fn FireProjectileClipSF
  (params (FireStructure :type Fire%20Structure%20Structure)))

(fn FireProjectileClipDPS
  (params (FireStructure :type Fire%20Structure%20Structure%20%28by%20ref%29)))

(fn FireProjectileNoClipSF
  (params (FireStructure :type Fire%20Structure%20Structure)))

(fn FireProjectileNoClipDPS
  (params (FireStructure :type Fire%20Structure%20Structure)))